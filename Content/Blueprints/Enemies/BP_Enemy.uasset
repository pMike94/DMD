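; BP_Enemy is an enemy actor that dies when hit by a TwinStickProjectile and awards points.
; On BeginPlay it caches the first BP_GameLogic actor found in the level.
; A projectile hit calls EnemyDeath, which adds KillValue to the game logic's Score, prints the total and destroys the enemy.
; The projectile's destruction is queued behind a short Delay that starts after the enemy has already destroyed itself.
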(event Collision|EventHit
  (params (MyComp :type Primitive%20Component%20Object%20Reference) (Other :type Actor%20Object%20Reference) (OtherComp :type Primitive%20Component%20Object%20Reference) (bSelfMoved :type Boolean) (HitLocation :type Vector :default "0, 0, 0") (HitNormal :type Vector :default "0, 0, 0") (NormalImpulse :type Vector :default "0, 0, 0") (Hit :type Hit%20Result%20Structure%20%28by%20ref%29))
  (bind _astwin_stick_projectile (Utilities|Casting|CastToTwinStickProjectile Other))
  (CallFunction|EnemyDeath)
  (Utilities|FlowControl|Delay 0.2)
  (Actor|DestroyActor _astwin_stick_projectile))

(event EventBeginPlay
  (bind _outactors (Actor|GetAllActorsOfClass "/Game/Blueprints/BP_GameLogic.BP_GameLogic_C"))
  (Variables|Default|SetGamelogic (Utilities|Array|Get(acopy) _outactors)))

(fn ConstructionScript)

(fn EnemyDeath
  (bind _gamelogic (Variables|Default|GetGamelogic))
  (bind _output_get (Variables|/Game/Blueprints/BP_GameLogic.BP_GameLogic_C|SetScore _gamelogic (+ (Variables|/Game/Blueprints/BP_GameLogic.BP_GameLogic_C|GetScore _gamelogic) (Variables|Default|GetKillValue))))
  (Development|PrintString (Utilities|String|ToString(Integer) _output_get))
  (Actor|DestroyActor))