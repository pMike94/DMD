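; Enemy AI controller that chases a TwinStickPawn.
; On BeginPlay it loops over all TwinStickPawn actors, measuring distance from the controller itself and storing any closer than the running Distance value as Target.
; Every Tick it calls SimpleMoveToActor toward that Target, which is chosen only once and never re-evaluated.
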(event EventTick
  (params (DeltaSeconds :type Float%20%28single-precision%29))
  (AI|Navigation|SimpleMovetoActor self (Variables|Default|GetTarget)))

(event EventBeginPlay
  (bind _outactors (Actor|GetAllActorsOfClass "/Game/TwinStickBP/Blueprints/TwinStickPawn.TwinStickPawn_C"))
  (for _array_element _outactors
    (if (< (Transformation|GetDistanceTo _array_element self) (Variables|Default|GetDistance))
      (Variables|Default|SetDistance (Transformation|GetDistanceTo _array_element self))
      (Variables|Default|SetTarget _array_element))))

(fn ConstructionScript)