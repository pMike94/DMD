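; BP_EnemySpawn is a spawner actor that spawns a set number of enemies over time at its own location.
; On BeginPlay it starts a looping timer at SpawnRate that calls SpawnEnemies.
; Each call spawns one EnemyType actor at the spawner's transform and decrements SpawnCount, clearing the timer by function name once the count runs out.
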(event EventBeginPlay
  (Utilities|Time|SetTimerbyFunctionName 0 "SpawnEnemies" (Variables|Default|GetSpawnRate) true))

(fn ConstructionScript)

(fn SpawnEnemies
  (if (> (Variables|Default|GetSpawnCount) 0)
    ;[1 1 1] Spawn Enemies until Spawn Count = 0
    (Game|SpawnActorfromClass (Variables|Default|GetEnemyType) (Transformation|GetActorTransform) "Undefined" 0 0)
    (Math|Integer|DecrementInt (Variables|Default|GetSpawnCount))
    (else
      (Utilities|Time|ClearTimerbyFunctionName self "SpawnEnemies"))))