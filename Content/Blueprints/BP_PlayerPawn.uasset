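; BP_PlayerPawn is the player-controlled pawn, with separate inputs for movement and facing.
; MoveForward and MoveRight add movement input along control-yaw forward and right vectors, ignoring pitch and roll to stay on the plane.
; FaceNorth and FaceEast share one node chain that sets the mesh's world rotation from a flat vector built from axis values.
; The left gamepad face button prints LocalID for debugging.
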(event EventBeginPlay)

(event Input|AxisEvents|InputAxisFaceNorth
  (params (AxisValue :type Float%20%28single-precision%29))
  ;[1 1 1] Rotation
  (Transformation|SetWorldRotation (Variables|Character|GetMesh) (Math|Conversions|RotationFromXVector (Math|Vector|MakeVector AxisValue (stale Input|AxisEvents|InputAxisFaceEast AxisValue) 0.0)) false false))

(event Input|AxisEvents|InputAxisFaceEast
  (params (AxisValue :type Float%20%28single-precision%29))
  ;[1 1 1] Rotation
  (Transformation|SetWorldRotation (Variables|Character|GetMesh) (Math|Conversions|RotationFromXVector (Math|Vector|MakeVector (stale Input|AxisEvents|InputAxisFaceNorth AxisValue) AxisValue 0.0)) false false))

(event Input|AxisEvents|InputAxisMoveForward
  (params (AxisValue :type Float%20%28single-precision%29))
  ;[1 1 1] Move
  (Pawn|Input|AddMovementInput (Math|Vector|GetForwardVector (Math|Rotator|MakeRotator 0.0 0.0 (.Yaw (Math|Rotator|BreakRotator (Pawn|GetControlRotation :!class /Script/Engine.Pawn))))) AxisValue false))

(event Input|AxisEvents|InputAxisMoveRight
  (params (AxisValue :type Float%20%28single-precision%29))
  ;[1 1 1] Move
  (Pawn|Input|AddMovementInput (Math|Vector|GetRightVector (Math|Rotator|MakeRotator 0.0 0.0 (.Yaw (Math|Rotator|BreakRotator (Pawn|GetControlRotation :!class /Script/Engine.Pawn))))) AxisValue false))

(event Input|GamepadEvents|GamepadFaceButtonLeft
  (params (Key :type Key%20Structure))
  ;[1 1 1] Debug Print own ID
  (:Pressed
    (Development|PrintString (Utilities|String|ToString(Integer) (Variables|Default|GetLocalID)))))

(fn ConstructionScript)